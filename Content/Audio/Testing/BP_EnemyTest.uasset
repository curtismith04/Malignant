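; BP_EnemyTest is a test actor in the audio testing folder that travels once along a spline from BeginPlay.
; A timeline, with play rate set to the inverse of Speed, maps its float to distance between the spline's start and last point.
; Each update moves the actor to that world location without sweeping and orients it along the tangent, which is sampled in local space.
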(event `self.ReceiveBeginPlay`
  (bind _spline (`self.Spline`))
  (`TimelineComponent.SetPlayRate` (`self.Timeline`) (/ 1.0 (`self.Speed`)))
  (bind (_direction _float) (`Timeline|Timeline` :!via `PlayFromStart`)
    (:`Update`
      (bind _returnvalue (`KismetMathLibrary.Lerp` 0.0 (`SplineComponent.GetDistanceAlongSplineAtSplinePoint` _spline (- (`SplineComponent.GetNumberOfSplinePoints` _spline) 1)) _float))
      (`self.K2_SetActorLocation` (`self.Actor`) (`SplineComponent.GetLocationAtDistanceAlongSpline` (`self.Spline`) _returnvalue "World") false false)
      (`self.K2_SetActorRotation` (`self.Actor`) (`KismetMathLibrary.Conv_VectorToRotator` (`SplineComponent.GetTangentAtDistanceAlongSpline` (`self.Spline`) _returnvalue "Local")) false))))

(fn `UserConstructionScript`)